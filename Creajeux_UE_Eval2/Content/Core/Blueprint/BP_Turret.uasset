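; BP_Turret is a turret that fires bullets and takes damage from them.
; While Detect is true, a Tick-driven Delay paces BP_Bullet spawns from the Billboard's transform; nothing here sets Detect.
; Bullets overlapping the Box cut HP; at zero it plays an explosion sound at world origin and a death effect, without destroying the actor.
; Tick also updates a WB_HealthBar widget and rotates it toward the player camera.
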(event `self.ReceiveTick`
  (params (DeltaSeconds :type "Float (single-precision)"))
  (`self.SpawnBullet`)
  (`self.HealthBarEvent`))

(event `SpawnBullet`
  (bind _billboard (`self.Billboard`))
  (if (`self.Detect`)
    (`KismetSystemLibrary.Delay` 0.5)
    (`|SpawnActorFromClass` "/Game/Core/Blueprint/BP_Bullet.BP_Bullet_C" (`KismetMathLibrary.MakeTransform` (`SceneComponent.K2_GetComponentLocation` _billboard) (`SceneComponent.K2_GetComponentRotation` _billboard)) "AlwaysSpawn" "MultiplyWithRoot" null null)))

(event `self.Box.OnComponentBeginOverlap`
  (params (OverlappedComponent :type "PrimitiveComponent Object Reference") (OtherActor :type "Actor Object Reference") (OtherComp :type "PrimitiveComponent Object Reference") (OtherBodyIndex :type Integer) (bFromSweep :type Boolean) (SweepResult :type "HitResult Structure (by ref)"))
  (cast `/Game/Core/Blueprint/BP_Bullet` OtherActor)
  (set `self.HP` (- (`self.HP`) 50.0))
  (if (<= (`self.HP`) 0.0)
    (`GameplayStatics.PlaySoundAtLocation` "/Game/Assets/Audio/Explode_Audio.Explode_Audio" (0.0 0.0 0.0) (struct) 1.0 1.0 0.0 null null null null)
    (`GameplayStatics.SpawnEmitterAttached` null (`self.P_DeathEffect`))))

(event `HealthBarEvent`
  (bind _healthbarwidget (`self.HealthBarWidget`))
  (bind _aswb_health_bar (cast `/Game/Core/Blueprint/WB_HealthBar` (`WidgetComponent.GetWidget` (`self.HealthBarWidget`))))
  (`ProgressBar.SetPercent` (`/Game/Core/Blueprint/WB_HealthBar.HealthBar` _aswb_health_bar) (/ (`self.HP`) 100.0))
  (`SceneComponent.K2_SetWorldRotation` _healthbarwidget (`KismetMathLibrary.FindLookAtRotation` (`SceneComponent.K2_GetComponentLocation` _healthbarwidget) (`SceneComponent.K2_GetComponentLocation` (`PlayerCameraManager.TransformComponent` (`GameplayStatics.GetPlayerCameraManager` 0)))) false false))

(fn `UserConstructionScript`)